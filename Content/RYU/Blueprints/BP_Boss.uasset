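; Boss character that tracks the player, takes hits from attack items and has an early draft of attack patterns.
; Overlapping a BP_AtkItem subtracts its Atk minus Def from HP; at low HP it jumps once and teleports to world origin.
; Tick uses a delay to periodically face the player, jumping when rotation changes.
; The charge movement is unconnected, and the commented fire-floor phase is not implemented.
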(event `self.ReceiveActorBeginOverlap`
  (params (OtherActor :type "Actor Object Reference"))
  ; 공격 받았을시 대미지 처리
  (bind _asbp_atk_item (cast `/Game/RYU/Blueprints/BP_AtkItem` OtherActor))
  (set `self.HP` (- (`self.HP`) (- (`/Game/RYU/Blueprints/BP_AtkItem.Atk` _asbp_atk_item) (`self.Def`))))
  ; 패턴3 - 체력이 반이하가 된 순간 중앙으로 점프 이후 불 장판
  (if (< (`self.HP`) 20)
    (`/Engine/EditorBlueprintResources/StandardMacros.DoOnce` false
      (:`Completed`
        (`self.Jump`)
        (`self.K2_SetActorLocation` (0.0 0.0 0.0))))))

(event `self.ReceiveTick`
  (params (DeltaSeconds :type "Float (single-precision)"))
  (bind (_returnvalue_roll _returnvalue_pitch) (`KismetMathLibrary.BreakRotator` (`self.K2_GetActorRotation`)))
  (bind _bossrotation (`self.BossRotation`))
  (bind (_returnvalue_roll_2 _returnvalue_pitch_2 _returnvalue_yaw) (`KismetMathLibrary.BreakRotator` (`KismetMathLibrary.FindLookAtRotation` (`self.K2_GetActorLocation`) (`self.PlayerLocation`))))
  ; 공격 후 1초 딜레이 후 플레이어를 바라본다
  (`KismetSystemLibrary.Delay` 1.0)
  (set `self.PlayerLocation` (`self.K2_GetActorLocation` (`GameplayStatics.GetPlayerCharacter` 0)))
  (bind _output_get (set `self.BossRotation` (`KismetMathLibrary.MakeRotator` _returnvalue_roll_2 _returnvalue_pitch _returnvalue_yaw)))
  (`self.K2_SetActorRotation` _output_get)
  ; 점프하며 방향 전환 (한번씩만 점프해야 하는데)
  (if (!= _bossrotation (`self.PreRotation`))
    (set `self.PreRotation` _bossrotation)
    (`/Engine/EditorBlueprintResources/StandardMacros.DoOnce` false :!label _label
      (:`Completed`
        (`self.Jump`)
        (goto _label :!via `Reset`)))))

(fn `UserConstructionScript`)