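; BP_TestLauncher is a test actor, apparently meant to spawn attack items on a left mouse click, as its comments describe.
; BeginPlay enables input from the first player controller, but no input event is wired.
; Two disconnected chains would spawn BP_AtkItem or BP_AtkItem2 at the player pawn's location, the first also making its StaticMesh transparent as a debug check.
; As it stands, nothing spawns.
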(event `self.ReceiveBeginPlay`
  ; 플레이어 컨트롤러 입력 받기
  (`self.EnableInput` (`GameplayStatics.GetPlayerController` 0)))

(event `Key|LeftMouseButton`
  (params (Key :type "Key Structure"))
  ; 마우스 좌클릭 시 아이템 스폰
)

(event `Key|RightMouseButton`
  (params (Key :type "Key Structure"))
  ; 마우스 좌클릭 시 아이템 스폰
)

(fn `UserConstructionScript`)