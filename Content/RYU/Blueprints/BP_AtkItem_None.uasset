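; BP_AtkItem_None is an attack item actor that spawns and launches like a projectile via the left mouse button.
; Pressing spawns another copy at the player pawn's location; releasing sets Click and switches TailEffect's material to M_Spark.
; While Click is true, Tick calls Move, shifting the actor along world +X at Speed, scaled by delta time, without sweep.
; The EnableInput and BP_TailEffect spawn nodes are disconnected and never run.
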(event `Key|LeftMouseButton`
  (params (Key :type "Key Structure"))
  ; 마우스 좌클릭 해방 시 click 체크
  (:`Released`
    (set `self.Click` true)
    ; TailEffect 머테리얼 이펙트로 변경
    (`PrimitiveComponent.SetMaterial` (`self.TailEffect`) 0 "/Game/StarterContent/Particles/Materials/M_Spark.M_Spark")))

(event `self.ReceiveBeginPlay`
  ; 플레이어 컨트롤러 입력 받기
)

(event `self.ReceiveTick`
  (params (DeltaSeconds :type "Float (single-precision)"))
  (if (`self.Click`)
    (`self.Move` (`self.K2_GetActorLocation`) (`KismetMathLibrary.GetForwardVector` (struct)) (`self.Speed`))))

(event `Key|LeftMouseButton`
  (params (Key :type "Key Structure"))
  ; 마우스 좌클릭 시 아이템 스폰
  (:`Pressed`
    (`|SpawnActorFromClass` "BP_AtkItem_None_C" (`KismetMathLibrary.MakeTransform` (`self.K2_GetActorLocation` (`GameplayStatics.GetPlayerPawn` 0))) "AlwaysSpawn" "MultiplyWithRoot" null null)))

(fn `Move`
  (params (Location :type "Vector Structure") (Direction :type "Vector Structure" :default (1.0 0.0 0.0)) (Speed :type "Float (double-precision)" :default 1.0))
  (`self.K2_SetActorLocation` (+ Location (* (* Direction Speed) (`GameplayStatics.GetWorldDeltaSeconds`)))))

(fn `UserConstructionScript`)