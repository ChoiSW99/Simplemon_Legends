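; BP_TailEffect is an actor that acts as a tail effect, continuously chasing a target actor.
; On BeginPlay it defaults the target to player pawn 0 if none is assigned.
; Each tick it feeds the normalized direction toward the target into a Move function, which offsets its location by speed times delta seconds, without sweep.
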(event `self.ReceiveBeginPlay`
  ; 꼬리가 쫓아갈 아이템이 지정되지 않았으면 디폴트로 쫓아갈 아이템 지정
  (`/Engine/EditorBlueprintResources/StandardMacros.IsValid` (`self.Target`)
    (:`Is Not Valid`
      (set `self.Target` (`GameplayStatics.GetPlayerPawn` 0)))))

(event `self.ReceiveTick`
  (params (DeltaSeconds :type "Float (single-precision)"))
  ; 꼬리가 타겟을 쫓아감
  (`self.Move` (`self.K2_GetActorLocation`) (`KismetMathLibrary.Normal` (- (`self.K2_GetActorLocation` (`self.Target`)) (`self.K2_GetActorLocation`))) (`self.Speed`)))

(fn `Move`
  (params (Location :type "Vector Structure") (Direction :type "Vector Structure" :default (1.0 0.0 0.0)) (Speed :type "Float (double-precision)" :default 1.0))
  (`self.K2_SetActorLocation` (+ Location (* (* Direction Speed) (`GameplayStatics.GetWorldDeltaSeconds`)))))

(fn `UserConstructionScript`)