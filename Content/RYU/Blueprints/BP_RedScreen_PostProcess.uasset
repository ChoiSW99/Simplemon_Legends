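; Post-process actor that applies the M_RedScreen material as a screen effect.
; On BeginPlay it creates a dynamic instance of that material and adds it to its PostProcess component as a full-weight blendable.
; Tick accumulates delta time into a looping timer that resets after about 20 seconds and feeds it to the material's Seconds scalar parameter to drive the effect over time.
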(event `self.ReceiveBeginPlay`
  (bind _returnvalue (`KismetMaterialLibrary.CreateDynamicMaterialInstance` "/Game/RYU/Meterials/M_RedScreen.M_RedScreen"))
  (bind _output_get (set `self.DynamicMaterial` _returnvalue))
  (`PostProcessComponent.AddOrUpdateBlendable` (`self.PostProcess`) _output_get 1.0))

(event `self.ReceiveTick`
  (params (DeltaSeconds :type "Float (single-precision)"))
  (bind _currenttime (`self.CurrentTime`))
  (if (> _currenttime 20.0)
    (set `self.CurrentTime` 0.0)
    (else
      (bind _output_get (set `self.CurrentTime` (+ _currenttime (`GameplayStatics.GetWorldDeltaSeconds`))))
      (if (> _output_get 0.0)
        (`MaterialInstanceDynamic.SetScalarParameterValue` (`self.DynamicMaterial`) "Seconds" _output_get)))))

(fn `UserConstructionScript`)