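; Boss character for the arena battle, with an opening walk-in and three attack patterns.
; Tick runs a flag-and-timer state machine that picks patterns by HP, randomness and position, and sets SwitchState.
; Patterns are an aimed charge, fireballs that players destroy to cause groggy or else face a firewall, and a half-HP center leap leaving a fire floor.
; Overlaps apply defense-reduced item damage, reporting HP to BattleGameMode, and charge damage to players.
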(event `StartGame`
  ; Enter 키 누르면 보스 움직임 시작
  (set `self.GameStart` true))

(event `self.ReceiveActorBeginOverlap`
  (params (OtherActor :type "Actor Object Reference"))
  (bind _ballcount (`self.BallCount`))
  (if (`self.GameStart`)
    (`|ExecutionSequence`
      (:`then_0`
        ; 공격 받았을시 대미지 처리
        (bind _asbp_atk_item (cast `/Game/RYU/Blueprints/BP_AtkItem` OtherActor))
        (if (`/Game/RYU/Blueprints/BP_AtkItem.Click` _asbp_atk_item)
          (`GameplayStatics.PlaySoundAtLocation` "/Game/StarterContent/Audio/Explosion02.Explosion02" (`self.K2_GetActorLocation`) (struct) 1.0 1.0 0.0 null null null null)
          ; 만약 패턴2 실행중이면 맞았을 시 화염구(꼬리)만 사라지고 대미지는 받지 않는다.
          (if (`self.Pattern2Loop`)
            (if (> _ballcount 0)
              ;; 화염구 하나 제거
              (`self.K2_DestroyActor` _asbp_atk_item)
              (bind _asbp_fire_ball (cast `/Game/RYU/Blueprints/Boss/BP_FireBall` (`|GetArrayItem` (`self.FireBallRef`) (- (`self.BallCount`) 1))))
              (`self.K2_DestroyActor` _asbp_fire_ball)
              (set `self.BallCount` (- _ballcount 1))
              ;; 패턴2 클리어
              (if (== (`self.BallCount`) 0)
                (`self.Pattern2`)))
            (else
              (bind _returnvalue (- (`/Game/RYU/Blueprints/BP_AtkItem.Atk` _asbp_atk_item) (`self.Def`)))
              (if (> _returnvalue 0)
                (bind _output_get (set `self.HP` (- (`self.HP`) _returnvalue)))
                (`/Game/CSW/BattleGameMode.UpdateBossHp` (`self.GameModeObj`) _output_get)
                (if (<= _output_get 0)
                  (set `self.IsEnd` true))
                (`self.K2_DestroyActor` _asbp_atk_item))))))
      (:`then_1`
        ; 패턴1 공격 중 접촉시 플레이어한테 대미지
        (if (`self.Pattern1Attack`)
          (bind _asbp_player_character (cast `/Game/CSW/Player/BP_PlayerCharacter` OtherActor))
          (`GameplayStatics.ApplyDamage` _asbp_player_character (`KismetMathLibrary.Conv_IntToDouble` (`self.Atk`))))))))

(event `self.ReceiveBeginPlay`
  (bind _maxhp (`self.MaxHP`))
  (bind _output_get (set `self.HP` _maxhp))
  (set `self.SwitchState` "NewEnumerator0")
  (bind _asbattle_game_mode (cast `/Game/CSW/BattleGameMode` (`GameplayStatics.GetGameMode`)))
  (bind _output_get_2 (set `self.GameModeObj` _asbattle_game_mode))
  (`/Game/CSW/BattleGameMode.SetBossMaxHp` _output_get_2 _maxhp)
  (`/Game/CSW/BattleGameMode.UpdateBossHp` _output_get_2 _output_get))

(event `self.ReceiveTick`
  (params (DeltaSeconds :type "Float (single-precision)"))
  (bind (_returnvalue_x _returnvalue_y _returnvalue_z) (`KismetMathLibrary.BreakVector` (`self.K2_GetActorLocation`)))
  (bind (_returnvalue_x_2 _returnvalue_y_2) (`KismetMathLibrary.BreakVector` (`self.K2_GetActorLocation`)))
  (bind _pattern1attack (`self.Pattern1Attack`))
  (bind _currenttime (`self.CurrentTime`))
  (bind _currenttime_2 (`self.CurrentTime`))
  (bind (_returnvalue_x_3 _returnvalue_y_3) (`KismetMathLibrary.BreakVector` (`self.K2_GetActorLocation` (`GameplayStatics.GetPlayerCharacter` 0))))
  (bind _returnvalue (* (* (`self.GetActorForwardVector`) (`self.WalkSpeed`)) (`GameplayStatics.GetWorldDeltaSeconds`)))
  (switch `int` (`self.Phase`)
    (:`Default`
      (`KismetSystemLibrary.PrintString` "이상한 페이즈가 입력되었습니다." true true (struct :`R` 1.0 :`A` 1.0)))
    (:`0`
      ; 오프닝 씬
      (if (`self.OpEnd`)
        (if (`|EnumInequality` (`self.SwitchState`) "NewEnumerator0")
          (if (> _currenttime 3.0)
            (set `self.CurrentTime` 0.0)
            (set `self.SwitchState` "NewEnumerator0")
            ;; 배틀맵으로 전환
            (set `self.Phase` 1)
            (else
              (set `self.CurrentTime` (+ _currenttime (`GameplayStatics.GetWorldDeltaSeconds`))))))
        (elif (`self.ArriveCenter`)
          (set `self.SwitchState` "NewEnumerator9")
          (set `self.OpEnd` true)
          (else
            ;; Idle2 애니메이션 -> Walk
            (if (`|EnumEquality` (`self.SwitchState`) "NewEnumerator7")
              (if (> _currenttime_2 4.0)
                (set `self.CurrentTime` 0.0)
                (set `self.SwitchState` "NewEnumerator8")
                (set `self.CenterDistance` (`KismetMathLibrary.Vector_Distance` (0.0 0.0 0.0) (`self.K2_GetActorLocation`)))
                (else
                  (set `self.CurrentTime` (+ _currenttime_2 (`GameplayStatics.GetWorldDeltaSeconds`)))))
              (elif (>= (`self.MoveDistance`) (`self.CenterDistance`))
                (set `self.ArriveCenter` true)
                (set `self.MoveDistance` 0.0)
                (else
                  ;; 필드 중앙까지 Walk -> ArriveCenter = true
                  (`self.K2_SetActorLocation` (+ (`self.K2_GetActorLocation`) _returnvalue))
                  (set `self.MoveDistance` (`KismetMathLibrary.VSize` _returnvalue)))))))))
    (:`1`
      (if (`self.GameStart`)
        ; 격파됨
        (if (`self.IsEnd`)
          (set `self.SwitchState` "NewEnumerator1")
          (elif (`self.IsJump`)
            ; 큰 점프가 종료되면
            (if (>= _returnvalue_z (- (`CharacterMovementComponent.GetMaxJumpHeight` (`self.CharacterMovement`)) 150.0))
              (set `self.SwitchState` "NewEnumerator11")
              (`self.LaunchCharacter` (- (0.0 0.0 0.0) (`self.K2_GetActorLocation`)))
              (else
                (`|ExecutionSequence`
                  (:`then_0`
                    (if (not (`NavMovementComponent.IsFalling` (`self.CharacterMovement`)))
                      (`self.JumpToCenter`)
                      (set `self.SwitchState` "NewEnumerator0")))
                  (:`then_1`
                    (if (and (`|EnumEquality` (`self.SwitchState`) "NewEnumerator11") (<= _returnvalue_z 400.0))
                      (set `self.SwitchState` "NewEnumerator6"))))))
            (elif (`self.JumpAttack`)
              ; 점프 이동 공격
              (if (< (`self.CurrentTime`) 2.0)
                (set `self.CurrentTime` (+ (`self.CurrentTime`) (`GameplayStatics.GetWorldDeltaSeconds`)))
                (else
                  (set `self.CurrentTime` 0.0)
                  (if (`self.Pattern3Attack`)
                    (`self.Pattern3`))
                  (set `self.JumpAttack` false)))
              (elif (`self.IsPattern`)
                (`|ExecutionSequence`
                  (:`then_0`
                    ; 패턴1 2초간 딜레이를 주면서 플레이어 세부 조준
                    (if (`self.Pattern1Loop`)
                      (if (< (`self.CurrentTime`) 2.0)
                        (set `self.CurrentTime` (+ (`self.CurrentTime`) (`GameplayStatics.GetWorldDeltaSeconds`)))
                        (`self.LookPlayer`)
                        (else
                          (set `self.CurrentTime` 0.0)
                          (`self.Pattern1`)))))
                  (:`then_1`
                    ; 패턴1 돌진 이동
                    (if _pattern1attack
                      ;; 한꺼번에 너무 이동하면 데드존 멀리 있는데 멈춰서 스피드를 낮추고 한 틱당 두번 이동
                      (`self.Run Attack`)
                      (if (and _pattern1attack (< (`self.MoveDistance`) (`self.RunDistance`)))
                        (`self.Run Attack`))))
                  (:`then_2`
                    ; 패턴2 화염구 대기 시간 (15초)
                    (if (`self.Pattern2Loop`)
                      (if (< (`self.CurrentTime`) 15.0)
                        (set `self.CurrentTime` (+ (`self.CurrentTime`) (`GameplayStatics.GetWorldDeltaSeconds`)))
                        (`|ExecutionSequence`
                          (:`then_0`
                            (if (and (> (`self.CurrentTime`) 1.0) (not (`self.RedScreen`)))
                              (set `self.RedScreen` true)
                              (bind _returnvalue_2 (`|SpawnActorFromClass` "/Game/RYU/Blueprints/BP_RedScreen_PostProcess.BP_RedScreen_PostProcess_C" (`KismetMathLibrary.MakeTransform` (0.0 0.0 0.0)) "Undefined" "MultiplyWithRoot" null null))
                              (set `self.RedScreenRef` _returnvalue_2)))
                          (:`then_1`
                            (if (and (> (`self.CurrentTime`) 13.0) (not (`self.ChargeEffect`)))
                              (set `self.ChargeEffect` true)
                              (bind _returnvalue_3 (`GameplayStatics.SpawnEmitterAttached` "/Game/FXVarietyPack/Particles/P_ky_lightning_custom.P_ky_lightning_custom" (`self.Effect`) "None" (0.0 0.0 0.0) (struct :`Pitch` 90.0) (0.5 0.5 0.5) "KeepRelativeOffset" false))
                              (set `self.BossEffect` _returnvalue_3)))
                          (:`then_2`
                            (if (and (> (`self.CurrentTime`) 11.0) (not (`self.CameraShakeMiddle`)))
                              (set `self.CameraShakeMiddle` true)
                              (`GameplayStatics.PlayWorldCameraShake` "/Game/RYU/Blueprints/BP_CameraShakeMiddle.BP_CameraShakeMiddle_C" (0.0 0.0 0.0) 0.0 10000.0))))
                        (else
                          (set `self.CurrentTime` 0.0)
                          (`self.Pattern2`)))))
                  (:`then_3`
                    ; 패턴3 하울링 모션 시간
                    (if (and (`self.Pattern3Attack`) (`|EnumEquality` (`self.SwitchState`) "NewEnumerator4"))
                      (if (< (`self.CurrentTime`) 2.0)
                        (set `self.CurrentTime` (+ (`self.CurrentTime`) (`GameplayStatics.GetWorldDeltaSeconds`)))
                        (else
                          (set `self.CurrentTime` 0.0)
                          (`self.Pattern3`))))))
                (else
                  ; 3초 그로기
                  (if (`self.IsGroggy`)
                    (if (< (`self.CurrentTime`) 3.0)
                      (set `self.Def` 0)
                      (set `self.CurrentTime` (+ (`self.CurrentTime`) (`GameplayStatics.GetWorldDeltaSeconds`)))
                      (else
                        (set `self.SwitchState` "NewEnumerator0")
                        (set `self.CurrentTime` 0.0)
                        (set `self.IsGroggy` false)
                        (set `self.Def` 2)))
                    (else
                      ; 패턴 끝난 직후 1초 딜레이
                      (if (`self.DelaySeconds`)
                        (if (< (`self.CurrentTime`) 1.0)
                          (set `self.CurrentTime` (+ (`self.CurrentTime`) (`GameplayStatics.GetWorldDeltaSeconds`)))
                          (else
                            (set `self.CurrentTime` 0.0)
                            (set `self.DelaySeconds` false)
                            ; 패턴 선택
                            (if (and (< (`self.HP`) (/ (`self.MaxHP`) 2)) (not (`self.Pattern3Attack`))) :!label _label
                              (`self.Pattern3`)
                              (elif (== (`self.HP`) (`self.MaxHP`))
                                (`self.Pattern1` :!label _label_2)
                                (elif (not (`self.Pattern1After`))
                                  (if (and (and (and (<= _returnvalue_x_3 200.0) (>= _returnvalue_x_3 -200.0)) (and (>= _returnvalue_y_3 -200.0) (<= _returnvalue_y_3 200.0))) (not (and (and (<= _returnvalue_x_2 200.0) (>= _returnvalue_x_2 -200.0)) (and (>= _returnvalue_y_2 -200.0) (<= _returnvalue_y_2 200.0))))) :!label _label_3
                                    (if (< (`KismetMathLibrary.RandomIntegerInRange` 0 9) 10)
                                      (`self.JumpToCenter`)
                                      (else
                                        (goto _label_2)))
                                    (else
                                      (goto _label_2)))
                                  (elif (< (`KismetMathLibrary.RandomIntegerInRange` 0 9) 3)
                                    (`self.Pattern2`)
                                    (else
                                      (goto _label_3))))))))
                        (else
                          (goto _label))))))))))))))

(event `Run Attack`
  (bind (_returnvalue_x _returnvalue_y) (`KismetMathLibrary.BreakVector` (- (`self.K2_GetActorLocation`) (`self.PreLocation`))))
  ; 패턴1 돌진 이동
  (if (< (`self.MoveDistance`) (`self.RunDistance`))
    (bind (_sweephitresult _returnvalue) (`self.K2_SetActorLocation` (+ (`self.K2_GetActorLocation`) (* (* (`KismetMathLibrary.Normal` (`KismetMathLibrary.GetForwardVector` (`self.BossRotation`))) (`self.Speed`)) (`GameplayStatics.GetWorldDeltaSeconds`))) true))
    (set `self.MoveDistance` (+ (`KismetMathLibrary.VSize` (`KismetMathLibrary.MakeVector` _returnvalue_x _returnvalue_y)) (`self.MoveDistance`)))
    ;; 데드존 부딪히면 돌진 종료
    (if (not _returnvalue)
      (set `self.SwitchState` "NewEnumerator0" :!label _label_4)
      (set `self.MoveDistance` 0.0)
      (`self.Pattern1`))
    (else
      (goto _label_4))))

(fn `EndPattern`
  (set `self.SwitchState` "NewEnumerator0")
  (set `self.DelaySeconds` true)
  (set `self.IsPattern` false)
  (set `self.IsGroggy` false))

(fn `GetPlayerDistance`
  (returns (Distance :type "Float (double-precision)"))
  (bind (_returnvalue_x _returnvalue_y) (`KismetMathLibrary.BreakVector` (- (`self.K2_GetActorLocation` (`GameplayStatics.GetPlayerCharacter` 0)) (`self.K2_GetActorLocation`))))
  (return (`KismetMathLibrary.VSize` (`KismetMathLibrary.MakeVector` _returnvalue_x _returnvalue_y))))

(fn `JumpOnce`
  ; 한번 점프
  (`/Engine/EditorBlueprintResources/StandardMacros.DoOnce` false
    (:`Completed`
      (`self.Jump`))))

(fn `JumpToCenter`
  (bind _charactermovement (`self.CharacterMovement`))
  (if (`self.IsJump`)
    (set `self.IsJump` false)
    (set `self.JumpAttack` true)
    (`|SpawnActorFromClass` "/Game/RYU/Blueprints/Boss/BP_ImpactFloor.BP_ImpactFloor_C" (`KismetMathLibrary.MakeTransform` (0.0 0.0 30.0)) "Undefined" "MultiplyWithRoot" null null)
    (`self.K2_SetActorLocation` (0.0 0.0 300.0))
    (set `CharacterMovementComponent.JumpZVelocity` 420.0 _charactermovement)
    (`GameplayStatics.PlayWorldCameraShake` "/Game/RYU/Blueprints/BP_CameraShakeLarge.BP_CameraShakeLarge_C" (0.0 0.0 0.0) 0.0 5000.0)
    (else
      (`self.LookCenter`)
      (set `self.IsJump` true)
      (set `self.SwitchState` "NewEnumerator5")
      (`/Engine/EditorBlueprintResources/StandardMacros.DoOnce` false
        (:`Completed`
          (set `CharacterMovementComponent.JumpZVelocity` 1500.0 _charactermovement)
          (`self.Jump`)
          (`self.LaunchCharacter` (+ (/ (- (0.0 0.0 0.0) (`self.K2_GetActorLocation`)) (`KismetMathLibrary.Conv_DoubleToVector` 2.0)) (`KismetMathLibrary.MakeVector` 0.0 0.0 (+ (`CharacterMovementComponent.GetMaxJumpHeight` (`self.CharacterMovement`)) 250.0)))))))))

(fn `LookCenter`
  (bind (_returnvalue_roll _returnvalue_pitch) (`KismetMathLibrary.BreakRotator` (`self.K2_GetActorRotation`)))
  (bind _bossrotation (`self.BossRotation`))
  (bind (_returnvalue_roll_2 _returnvalue_pitch_2 _returnvalue_yaw) (`KismetMathLibrary.BreakRotator` (`KismetMathLibrary.FindLookAtRotation` (`self.K2_GetActorLocation`) (0.0 0.0 0.0))))
  ; 필드 중앙으로 몸을 돌린다
  (bind _output_get (set `self.BossRotation` (`KismetMathLibrary.MakeRotator` _returnvalue_roll_2 _returnvalue_pitch _returnvalue_yaw)))
  (`self.K2_SetActorRotation` _output_get)
  ; 방향 정보 저장
  (if (!= _bossrotation (`self.PreRotation`))
    (set `self.PreRotation` _bossrotation)))

(fn `LookPlayer`
  (bind (_returnvalue_roll _returnvalue_pitch) (`KismetMathLibrary.BreakRotator` (`self.K2_GetActorRotation`)))
  (bind _bossrotation (`self.BossRotation`))
  (bind (_returnvalue_roll_2 _returnvalue_pitch_2 _returnvalue_yaw) (`KismetMathLibrary.BreakRotator` (`KismetMathLibrary.FindLookAtRotation` (`self.K2_GetActorLocation`) (`self.PlayerLocation`))))
  ; 플레이어 방향으로 몸을 돌린다
  (set `self.PlayerLocation` (`self.K2_GetActorLocation` (`GameplayStatics.GetPlayerCharacter` 0)))
  (bind _output_get (set `self.BossRotation` (`KismetMathLibrary.MakeRotator` _returnvalue_roll_2 _returnvalue_pitch _returnvalue_yaw)))
  (`self.K2_SetActorRotation` _output_get)
  ; 방향 정보 저장
  (if (!= _bossrotation (`self.PreRotation`))
    (set `self.PreRotation` _bossrotation)))

(fn `Pattern1`
  (if (`self.IsJump`)
    _
    (elif (`self.Pattern1Attack`)
      ; 앞으로 돌진 (애니메이션 적용)
      (`ActorComponent.K2_DestroyComponent` (`self.BossEffect`))
      (set `self.Pattern1Attack` false)
      ; 패턴 완료
      (`self.EndPattern`)
      (elif (`self.Pattern1Loop`)
        (set `self.Pattern1Loop` false)
        (set `self.Pattern1Attack` true)
        (set `self.SwitchState` "NewEnumerator2")
        (set `self.PreLocation` (`self.K2_GetActorLocation`))
        (bind _returnvalue (`GameplayStatics.SpawnEmitterAttached` "/Game/FXVarietyPack/Particles/P_ky_lightning_custom.P_ky_lightning_custom" (`self.Effect`) "None" (0.0 0.0 0.0) (struct :`Pitch` 90.0) (0.5 0.5 0.5) "KeepRelativeOffset" false))
        (set `self.BossEffect` _returnvalue)
        (else
          (set `self.IsPattern` true)
          (set `self.Pattern1After` true)
          ; 플레이어를 바라본다
          (`self.LookPlayer`)
          (`self.JumpOnce`)
          (if (not (`self.Pattern1Loop`))
            (set `self.Pattern1Loop` true)))))))

(fn `Pattern2`
  (bind _bossrotation (`self.BossRotation`))
  (bind _bosseffect (`self.BossEffect`))
  (bind (_returnvalue_x _returnvalue_y) (`KismetMathLibrary.BreakVector` (`self.K2_GetActorLocation` (`GameplayStatics.GetPlayerCharacter` 0))))
  (if (not (`self.IsJump`))
    (set `self.IsPattern` true)
    (if (`self.Pattern2Loop`)
      (`/Engine/EditorBlueprintResources/StandardMacros.IsValid` _bosseffect
        (:`Is Valid`
          (`ActorComponent.K2_DestroyComponent` _bosseffect))
        (:`Is Not Valid`
          _))
      (set `self.ChargeEffect` false)
      (set `self.CurrentTime` 0.0)
      ; 루프 종료 후 BallCount 가 남아있으면 불기둥 생성
      (set `self.Pattern2Loop` false)
      (`KismetArrayLibrary.Array_Clear` (`self.FireBallRef`))
      (if (> (`self.BallCount`) 0)
        (`|SpawnActorFromClass` "/Game/RYU/Blueprints/Boss/BP_FireWall.BP_FireWall_C" (`KismetMathLibrary.MakeTransform` (`KismetMathLibrary.MakeVector` _returnvalue_x _returnvalue_y 200.0)) "Undefined" "MultiplyWithRoot" null null))
      (`self.K2_DestroyActor` (`self.RedScreenRef`))
      (set `self.RedScreen` false)
      (set `self.CameraShakeMiddle` false)
      ; 패턴 완료
      (`self.EndPattern`)
      ; 패턴2 루프 종료 후 BallCount 가 0 이면 그로기
      (if (== (`self.BallCount`) 0)
        (set `self.IsGroggy` true)
        (set `self.SwitchState` "NewEnumerator3")
        (else
          (set `self.BallCount` 0)))
      (else
        (set `self.Pattern1After` false)
        (`self.LookPlayer`)
        ; 화염구 5개 생성 (spawn)
        (set `self.BallCount` 5)
        (for _index (range -2 3)
          (bind (_returnvalue_x_2 _returnvalue_y_2) (`KismetMathLibrary.BreakVector` (+ (`self.K2_GetActorLocation`) (+ (* (* _index 70) (`KismetMathLibrary.Normal` (`KismetMathLibrary.GetRightVector` _bossrotation))) (* (`KismetMathLibrary.Normal` (`KismetMathLibrary.GetForwardVector` _bossrotation)) (`KismetMathLibrary.Conv_IntToVector` 250))))))
          (bind _returnvalue (`|SpawnActorFromClass` "/Game/RYU/Blueprints/Boss/BP_FireBall.BP_FireBall_C" (`KismetMathLibrary.MakeTransform` (`KismetMathLibrary.MakeVector` _returnvalue_x_2 _returnvalue_y_2 (- (`KismetMathLibrary.Conv_IntToDouble` 500) (* (`KismetMathLibrary.Abs_Int` _index) 10))) _bossrotation) "Undefined" "MultiplyWithRoot" null null))
          (`KismetArrayLibrary.Array_Add` (`self.FireBallRef`) _returnvalue))
        (set `self.Pattern2Loop` true)))))

(fn `Pattern3`
  (if (`self.Pattern3Attack`)
    ; 중앙으로 점프 이후 불 장판
    (if (`self.JumpAttack`)
      (`|SpawnActorFromClass` "/Game/RYU/Blueprints/Boss/BP_FireFloor.BP_FireFloor_C" (`KismetMathLibrary.MakeTransform` (0.0 0.0 10.0)) "Undefined" "MultiplyWithRoot" null null)
      ; 패턴 완료
      (`self.EndPattern`)
      (else
        (`self.JumpToCenter`)))
    (else
      (set `self.IsPattern` true)
      (set `self.Pattern1After` false)
      (`self.LookCenter`)
      (`self.JumpOnce`)
      (set `self.Pattern3Attack` true)
      (set `self.SwitchState` "NewEnumerator4"))))

(fn `UserConstructionScript`)