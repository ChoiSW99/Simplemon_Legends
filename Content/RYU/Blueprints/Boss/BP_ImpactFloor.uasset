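; BP_ImpactFloor is a boss hazard actor that marks a floor spot with smoke and damages the player on contact.
; BeginPlay spawns a P_Smoke emitter at its location, and overlap with BP_PlayerCharacter applies damage equal to its Atk value.
; Tick accumulates delta time until Life is reached, then destroys both the emitter and the actor.
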(event `self.ReceiveBeginPlay`
  (bind _returnvalue (`GameplayStatics.SpawnEmitterAtLocation` "/Game/StarterContent/Particles/P_Smoke.P_Smoke" (`self.K2_GetActorLocation`))))

(event `self.ReceiveActorBeginOverlap`
  (params (OtherActor :type "Actor Object Reference"))
  ; 플레이어한테 대미지
  (bind _asbp_player_character (cast `/Game/CSW/Player/BP_PlayerCharacter` OtherActor))
  (`GameplayStatics.ApplyDamage` _asbp_player_character (`KismetMathLibrary.Conv_IntToDouble` (`self.Atk`))))

(event `self.ReceiveTick`
  (params (DeltaSeconds :type "Float (single-precision)"))
  ; 만들어진지 일정 시간 지나면 사라진다
  (if (< (`self.CurrentTime`) (`self.Life`))
    (set `self.CurrentTime` (+ (`self.CurrentTime`) (`GameplayStatics.GetWorldDeltaSeconds`)))
    (else
      (set `self.CurrentTime` 0.0)
      (`ActorComponent.K2_DestroyComponent` (stale `self.ReceiveBeginPlay` _returnvalue))
      (`self.K2_DestroyActor`))))

(fn `UserConstructionScript`)