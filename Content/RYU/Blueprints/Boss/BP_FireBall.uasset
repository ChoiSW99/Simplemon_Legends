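; Boss fireball actor that shows a fire effect and removes itself after a set lifetime.
; BeginPlay spawns the P_Fire emitter at the actor's location, unattached.
; Tick accumulates delta time until it reaches Life, then resets the counter and destroys the actor.
; It has no overlap or damage logic; a note assigns the countdown and fire-pillar summon to the boss logic.
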(event `self.ReceiveBeginPlay`
  (`GameplayStatics.SpawnEmitterAtLocation` "/Game/StarterContent/Particles/P_Fire.P_Fire" (`self.K2_GetActorLocation`)))

(event `self.ReceiveTick`
  (params (DeltaSeconds :type "Float (single-precision)"))
  ; 15초가 지나면 불기둥을 소환하고 자동으로 사라진다 / 카운트 및 불기둥은 보스 로직
  (if (< (`self.CurrentTime`) (`self.Life`))
    (set `self.CurrentTime` (+ (`self.CurrentTime`) (`GameplayStatics.GetWorldDeltaSeconds`)))
    (else
      (set `self.CurrentTime` 0.0)
      (`self.K2_DestroyActor`))))

(fn `UserConstructionScript`)