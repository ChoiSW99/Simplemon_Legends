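; BP_AtkItem is a thrown attack item that launches when the left mouse button is released, swapping its tail effect material.
; Tick first moves it manually toward a virtual point ahead of the player camera.
; Once that distance is covered, it activates ProjectileMovement along the captured camera direction, so the shot follows the aim line.
; Overlapping BP_Boss spawns an explosion emitter; no damage or destruction happens here.
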(event `self.ReceiveTick`
  (params (DeltaSeconds :type "Float (single-precision)"))
  (bind _projectilemovement (`self.ProjectileMovement`))
  (bind _returnvalue (* (* (* (`self.Speed`) 1.2) (`self.TergetDirection`)) (`GameplayStatics.GetWorldDeltaSeconds`)))
  (if (`self.IsEnd`)
    _
    (elif (`self.Click`)
      ; 방향 설정
      (if (`self.IsFly`)
        ; Target Direction 의 x 축 + 100 위치까지 set actor location 으로 반복 이동
        (if (>= (`self.Distance`) (`self.TargetDistance`))
          ; 타겟 조준 위치로 projectileMovement
          (set `MovementComponent.Velocity` (* (`self.Speed`) (`self.CameraDirection`)) _projectilemovement)
          (`ActorComponent.Activate` _projectilemovement false)
          (set `self.IsEnd` true)
          (else
            (set `self.Distance` (+ (`self.Distance`) (`KismetMathLibrary.VSize` _returnvalue)))
            (`self.K2_SetActorLocation` (+ _returnvalue (`self.K2_GetActorLocation`)))))
        (else
          ;; 3인칭 캐릭터 카메라
          (bind _asbp_player_character (cast `/Game/CSW/Player/BP_PlayerCharacter` (`GameplayStatics.GetPlayerCharacter` 0)))
          (bind _camera (`/Game/CSW/Player/BP_PlayerCharacter.Camera` _asbp_player_character))
          (bind _returnvalue_2 (`KismetMathLibrary.Normal` (`SceneComponent.GetForwardVector` _camera)))
          (bind _returnvalue_3 (- (+ (`SceneComponent.K2_GetComponentLocation` _camera) (* _returnvalue_2 (`KismetMathLibrary.Conv_DoubleToVector` 700.0))) (`self.K2_GetActorLocation`)))
          (set `self.TargetDistance` (`KismetMathLibrary.VSize` _returnvalue_3))
          (set `self.TergetDirection` (`KismetMathLibrary.Normal` _returnvalue_3))
          (set `self.CameraDirection` _returnvalue_2)
          (set `self.IsFly` true))))))

(event `self.ReceiveActorBeginOverlap`
  (params (OtherActor :type "Actor Object Reference"))
  ; 아이템 충돌 시 플레이어가 아닐 경우 아이템 소멸 이펙트 (몬스터는 아이템에 맞을 경우 데미지)
  (cast `/Game/RYU/Blueprints/Boss/BP_Boss` OtherActor)
  (`GameplayStatics.SpawnEmitterAtLocation` "/Game/StarterContent/Particles/P_Explosion.P_Explosion" (`self.K2_GetActorLocation`)))

(event `Key|LeftMouseButton`
  (params (Key :type "Key Structure"))
  ; 마우스 좌클릭 해방 시 click 체크
  (:`Released`
    (set `self.Click` true)
    ; TailEffect 머테리얼 이펙트로 변경
    (`PrimitiveComponent.SetMaterial` (`self.TailEffect`) 0 "/Game/StarterContent/Particles/Materials/M_Spark.M_Spark")))

(event `self.ReceiveBeginPlay`
  ; 플레이어 컨트롤러 입력 받기
  (`self.EnableInput` (`GameplayStatics.GetPlayerController` 0)))

(fn `Move`
  (params (Location :type "Vector Structure") (Direction :type "Vector Structure" :default (1.0 0.0 0.0)) (Speed :type "Float (double-precision)" :default 1.0))
  (`self.K2_SetActorLocation` (+ Location (* (* Direction Speed) (`GameplayStatics.GetWorldDeltaSeconds`)))))

(fn `UserConstructionScript`)